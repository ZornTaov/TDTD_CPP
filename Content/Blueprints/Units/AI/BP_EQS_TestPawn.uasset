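; BP_EQS_TestPawn is a test pawn, named for Environment Query System work, that runs the base unit AI behavior tree.
; On BeginPlay its AI controller starts BT_BaseUnitAI.
; Every tick it writes the world location of its Arrow1 component into a blackboard vector key, feeding the tree a position that follows the arrow.
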(event `self.ReceiveBeginPlay`
  (`AIController.RunBehaviorTree` (`AIBlueprintHelperLibrary.GetAIController` self) "/Game/Blueprints/Units/AI/BT_BaseUnitAI.BT_BaseUnitAI"))

(event `self.ReceiveTick`
  (params (DeltaSeconds :type "Float (single-precision)"))
  (`BlackboardComponent.SetValueAsVector` (`AIBlueprintHelperLibrary.GetBlackboard` (`AIBlueprintHelperLibrary.GetAIController` self)) (`self.Key Name`) (`SceneComponent.K2_GetComponentLocation` (`self.Arrow1`))))

(fn `UserConstructionScript`)